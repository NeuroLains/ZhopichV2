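; Alien enemy that wanders around its spawn point and is destroyed when its health runs out.
; BeginPlay stores the start location, fills health and starts a patrol loop issuing AI moves to random reachable points within a radius.
; The loop waits a random delay after issuing each move, without waiting for arrival.
; Damage lowers clamped health, and Tick polls it to trigger death.
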(event Custom|DeathC
  ;[1 1 1] Death
  (Variables|Default|SetDeath true)
  (Variables|Default|SetAlive false)
  (Actor|DestroyActor))

(event Custom|StartPatrolling
  ;[1 1 1] Patrol
  (if (Variables|Default|GetAlive) :!label _label
    (AI|AIMoveTo self (.RandomLocation (AI|Navigation|GetRandomReachablePointinRadius (Variables|Default|GetStartingLocation) (Variables|Default|GetPatrolRadius) 0 0)) 0 2e+01 false
      (:then
        (Utilities|FlowControl|Delay (Math|Random|RandomFloatinRange (Variables|Default|GetPatrolDelayMin) (Variables|Default|GetPatrolDelayMax)))
        (goto _label)))))

(event Custom|InitHealt
  ;[1 1 1] Health
  (Variables|Default|SetHealth (Variables|Default|GetMaxHealth)))

(event EventBeginPlay
  ;[1 1 1] BeginPlay
  (Variables|Default|SetStartingLocation (Transformation|GetActorLocation))
  (CallFunction|StartPatrolling)
  (CallFunction|InitHealt)
  (Variables|Default|SetAlive true))

(event Game|Damage|EventAnyDamage
  (params (Damage :type Float%20%28single-precision%29) (DamageType :type Damage%20Type%20Object%20Reference) (InstigatedBy :type Controller%20Object%20Reference) (DamageCauser :type Actor%20Object%20Reference))
  ;[1 1 1] Damage
  (if (not (Variables|Default|GetDeath))
    (Variables|Default|SetHealth (Math|Float|Clamp(Float) (- (Variables|Default|GetHealth) Damage) 0.0 (Variables|Default|GetMaxHealth)))))

(event EventTick
  (params (DeltaSeconds :type Float%20%28single-precision%29))
  ;[1 1 1] Tick
  (if (<= (Variables|Default|GetHealth) 0.0)
    (CallFunction|DeathC)))

(fn ConstructionScript)