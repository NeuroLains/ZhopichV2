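; BP_Turel is an enemy turret that uses PawnSensing to spot pawns and fire at them while enabled.
; It snaps its whole actor rotation toward a sighted BP_Zhopich, but queues a shot for any seen pawn.
; A Delay of Speed paces fire, then Shot spawns BP_DIldoEnemy at the Shoot component's transform.
; IsEnable and IsDisable toggle the turret, and debug strings print on each sighting.
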(event OnSeePawn(PawnSensing)
  (params (Pawn :type Pawn%20Object%20Reference))
  (if (Variables|Default|GetEnable)
    (Utilities|FlowControl|Sequence
      (:then_0
        (bind _asbp_zhopich (Utilities|Casting|CastToBP_Zhopich Pawn)
          (:then
            (Development|PrintString "Vis")
            (Transformation|SetActorRotation (Math|Rotator|FindLookatRotation (Transformation|GetActorLocation) (Transformation|GetWorldLocation (Variables|/Script/Engine.Actor|GetRootComponent _asbp_zhopich)))))
          (:CastFailed
            (Development|PrintString "stealyh"))))
      (:then_1
        (Utilities|FlowControl|Delay (Variables|Default|GetSpeed))
        (CallFunction|Shot)))))

(event Custom|IsDisable
  (Variables|Default|SetEnable false))

(event Custom|IsEnable
  (Variables|Default|SetEnable true))

(event Custom|Shot
  ;[1 1 1] Shot
  (Game|SpawnActorfromClass "/Game/Alien/Blueprint/Bullet/BP_DIldoEnemy.BP_DIldoEnemy_C" (Transformation|GetWorldTransform (Variables|Default|GetShoot)) "AlwaysSpawn" "MultiplyWithRoot" 0 0))

(event EventBeginPlay)

(event Collision|EventActorBeginOverlap
  (params (OtherActor :type Actor%20Object%20Reference)))

(event EventTick
  (params (DeltaSeconds :type Float%20%28single-precision%29)))

(fn ConstructionScript)