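; SimpleMovingObject is a Blueprint that moves a static mesh back and forth along the Track spline, pausing at each end.
; Tick advances a clamped movement time by the direction, then at either end flips direction and waits before resuming.
; A float curve remaps normalized time for easing before the spline is sampled for the mesh's world location.
; The construction script sets track duration and places the mesh at its configured start position.
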(event EventTick
  (params (DeltaSeconds :type Float%20%28single-precision%29))
  (Variables|Default|SetDeltaSeconds DeltaSeconds)
  (if (Variables|Default|GetCanMove)
    (Variables|Default|SetMovementTime (Math|Float|Clamp(Float) (+ (Variables|Default|GetMovementTime) (* (Variables|MovementParameters|GetMovementDirection) (Variables|Default|GetDeltaSeconds))) 0.0 (Variables|/Script/Engine.SplineComponent|GetDuration (Variables|Default|GetTrack))))
    (Math|Integer|CompareInt (Variables|MovementParameters|GetMovementDirection)
      (:>
        (if (Math|Float|NearlyEqual(Float) (Variables|/Script/Engine.SplineComponent|GetDuration (Variables|Default|GetTrack)) (Variables|Default|GetMovementTime) 1e-06)
          (Variables|Default|SetCanMove false :!label _label)
          (Variables|MovementParameters|SetMovementDirection (* (Variables|MovementParameters|GetMovementDirection) -1))
          (Utilities|FlowControl|Delay (Variables|MovementParameters|GetWaitTime))
          (Variables|Default|SetCanMove true)
          (else
            (CallFunction|UpdateObjectLocation :!label _label_2))))
      (:<
        (if (Math|Float|NearlyEqual(Float) 0.0 (Variables|Default|GetMovementTime) 1e-06)
          (goto _label)
          (else
            (goto _label_2)))))))

(fn ConstructionScript
  (|CallParentFunction)
  (Variables|/Script/Engine.SplineComponent|SetDuration (Variables|Default|GetTrack) (Variables|MovementParameters|GetMovementDuration))
  (Variables|Default|SetMovementTime (* (Variables|MovementParameters|GetMovementDuration) (Variables|MovementParameters|GetStartPosition)))
  (CallFunction|UpdateObjectLocation))

(fn UpdateObjectLocation
  (bind _track (Variables|Default|GetTrack))
  (bind _duration (Variables|/Script/Engine.SplineComponent|GetDuration _track))
  (Transformation|SetWorldLocation (Variables|Default|GetStaticMesh) (Spline|GetLocationatTime (Variables|Default|GetTrack) (Math|Float|MapRangeClamped (Math|Curves|GetFloatValue (Variables|MovementParameters|GetMovementCurve) (Math|Float|NormalizetoRange (Variables|Default|GetMovementTime) 0.0 _duration)) 0.0 1.0 0.0 _duration) "World" false) false false))