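; SimpleObjectBuilder is a configurable mesh Blueprint that builds a styled object from its Mesh, Material, color and surface variables.
; Its construction script assigns the mesh to a StaticMesh component and sets the material on slot zero.
; It then pushes top and side color pairs, tiling and roughness into material parameters, so one material supports differently styled copies.
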(fn ConstructionScript
  (Components|StaticMesh|SetStaticMesh (Variables|Default|GetStaticMesh) (Variables|MeshParameters|GetMesh))
  (Rendering|Material|SetMaterial (Variables|Default|GetStaticMesh) 0 (Variables|MeshParameters|GetMaterial))
  (Rendering|Material|SetVectorParameterValueonMaterials (Variables|Default|GetStaticMesh) "TopColor_1" (Math|Conversions|ToVector(LinearColor) (Variables|MeshParameters|GetTopColor%201)))
  (Rendering|Material|SetVectorParameterValueonMaterials (Variables|Default|GetStaticMesh) "TopColor_2" (Math|Conversions|ToVector(LinearColor) (Variables|MeshParameters|GetTopColor%202)))
  (Rendering|Material|SetVectorParameterValueonMaterials (Variables|Default|GetStaticMesh) "SideColor_1" (Math|Conversions|ToVector(LinearColor) (Variables|MeshParameters|GetSideColor%201)))
  (Rendering|Material|SetVectorParameterValueonMaterials (Variables|Default|GetStaticMesh) "SideColor_2" (Math|Conversions|ToVector(LinearColor) (Variables|MeshParameters|GetSideColor%202)))
  (Rendering|Material|SetScalarParameterValueonMaterials (Variables|Default|GetStaticMesh) "Tiling" (Variables|MeshParameters|GetTiling))
  (Rendering|Material|SetScalarParameterValueonMaterials (Variables|Default|GetStaticMesh) "Roughness" (Variables|MeshParameters|GetRoughness)))