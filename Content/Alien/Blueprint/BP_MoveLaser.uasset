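; BP_MoveLaser is an actor that moves a cylinder, by its name a laser, back and forth along the Track spline.
; Tick advances a clamped movement time, pausing at each end for a wait time before reversing direction.
; UpdateObjectLocation remaps that time through a float curve to shape motion along the spline.
; The construction script sets spline duration and places the cylinder at its configurable start position.
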(event EventBeginPlay
  (|CallParentFunction) ; Этот узел отключен и не будет вызываться.\nПеретащите контакты, чтобы построить функционал.
)

(event EventTick
  (params (DeltaSeconds :type Float%20%28single-precision%29))
  (bind _output_get (Variables|Default|SetDeltaSeconds DeltaSeconds))
  (|CallParentFunction _output_get)
  (if (Variables|Default|GetCanMove)
    (Variables|Default|SetMovementTime (Math|Float|Clamp(Float) (+ (Variables|Default|GetMovementTime) (* (Variables|Default|GetMovementDirection) (Variables|Default|GetDeltaSeconds))) 0.0 (Variables|/Script/Engine.SplineComponent|GetDuration (Variables|Default|GetTrack))))
    (Math|Integer|CompareInt (Variables|Default|GetMovementDirection)
      (:>
        (if (Math|Float|NearlyEqual(Float) (Variables|/Script/Engine.SplineComponent|GetDuration (Variables|Default|GetTrack)) (Variables|Default|GetMovementTime) 1e-06)
          (Variables|Default|SetCanMove false :!label _label)
          (Variables|Default|SetMovementDirection (* (Variables|Default|GetMovementDirection) -1))
          (Utilities|FlowControl|Delay (Variables|Default|GetWaitTime))
          (Variables|Default|SetCanMove true)
          (else
            (CallFunction|UpdateObjectLocation :!label _label_2))))
      (:<
        (if (Math|Float|NearlyEqual(Float) 0.0 (Variables|Default|GetMovementTime) 1e-06)
          (goto _label)
          (else
            (goto _label_2)))))))

(event Collision|EventActorBeginOverlap
  (params (OtherActor :type Actor%20Object%20Reference))
  (|CallParentFunction OtherActor) ; Этот узел отключен и не будет вызываться.\nПеретащите контакты, чтобы построить функционал.
)

(fn ConstructionScript
  (|CallParentFunction)
  (Variables|/Script/Engine.SplineComponent|SetDuration (Variables|Default|GetTrack) (Variables|Default|GetMovementDuration))
  (Variables|Default|SetMovementTime (* (Variables|Default|GetMovementDuration) (Variables|Default|GetStartPosition)))
  (CallFunction|UpdateObjectLocation))

(fn UpdateObjectLocation
  (bind _track (Variables|Default|GetTrack))
  (bind _duration (Variables|/Script/Engine.SplineComponent|GetDuration _track))
  (Transformation|SetWorldLocation (Variables|Default|GetCylinder) (Spline|GetLocationatTime (Variables|Default|GetTrack) (Math|Float|MapRangeClamped (Math|Curves|GetFloatValue (Variables|Default|GetMovementCurve) (Math|Float|NormalizetoRange (Variables|Default|GetMovementTime) 0.0 _duration)) 0.0 1.0 0.0 _duration) "World" false) false false))