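; BP_Rat is an enemy rat that chases and bites the player.
; Its PawnSensing component sets a seen-player flag and starts an AI MoveTo toward the player character.
; Because the flag is set just before its check, the delayed StartPatrolling branch never runs from that event.
; Once the flag is set, BP_Character overlaps with its sphere deal damage to the player after a short delay and print a debug bite message.
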(event OnSeePawn(PawnSensing)
  (params (Pawn :type Pawn%20Object%20Reference))
  ;[1 1 1] See player
  (bind _output_get (Variables|Default|SetisSeePlayer true))
  (if _output_get
    (CallFunction|FollowPlayer)
    (else
      (Utilities|FlowControl|Delay 1.0)
      (CallFunction|StartPatrolling))))

(event OnComponentBeginOverlap(Sphere)
  (params (OverlappedComponent :type Primitive%20Component%20Object%20Reference) (OtherActor :type Actor%20Object%20Reference) (OtherComp :type Primitive%20Component%20Object%20Reference) (OtherBodyIndex :type Integer) (bFromSweep :type Boolean) (SweepResult :type Hit%20Result%20Structure%20%28by%20ref%29))
  ;[1 1 1] Damage
  (Utilities|Casting|CastToBP_Character OtherActor)
  (if (Variables|Default|GetisSeePlayer)
    (Utilities|FlowControl|Delay 0.1)
    (Game|Damage|ApplyDamage (Game|GetPlayerCharacter 0) 4e+01 0 0)
    (Development|PrintString "KUS-KUS")))

(event Custom|FollowPlayer
  ;[1 1 1] Follow
  (AI|AIMoveTo self "0, 0, 0" (Game|GetPlayerCharacter 0) 5.0 false))

(event EventBeginPlay
  (|CallParentFunction) ; Этот узел отключен и не будет вызываться.\nПеретащите контакты, чтобы построить функционал.
)

(event Collision|EventActorBeginOverlap
  (params (OtherActor :type Actor%20Object%20Reference)))

(event EventTick
  (params (DeltaSeconds :type Float%20%28single-precision%29))
  (|CallParentFunction DeltaSeconds) ; Этот узел отключен и не будет вызываться.\nПеретащите контакты, чтобы построить функционал.
)

(fn ConstructionScript
  (|CallParentFunction))