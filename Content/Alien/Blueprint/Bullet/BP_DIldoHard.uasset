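; Bullet actor that damages enemies and copters and destroys itself after a short lifespan.
; Sphere overlaps cast the other actor to BP_Enemy and BP_Copter in sequence, applying the same fixed damage with the first player controller as instigator.
; Sphere hits call BreakItemMessage on the struck actor to signal breakable items.
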(event OnComponentHit(Sphere)
  (params (HitComponent :type Primitive%20Component%20Object%20Reference) (OtherActor :type Actor%20Object%20Reference) (OtherComp :type Primitive%20Component%20Object%20Reference) (NormalImpulse :type Vector :default "0, 0, 0") (Hit :type Hit%20Result%20Structure%20%28by%20ref%29))
  (Class|BPIInteraction|BreakItem(Message) (.HitActor (Collision|BreakHitResult Hit))))

(event OnComponentBeginOverlap(Sphere)
  (params (OverlappedComponent :type Primitive%20Component%20Object%20Reference) (OtherActor :type Actor%20Object%20Reference) (OtherComp :type Primitive%20Component%20Object%20Reference) (OtherBodyIndex :type Integer) (bFromSweep :type Boolean) (SweepResult :type Hit%20Result%20Structure%20%28by%20ref%29))
  (Utilities|FlowControl|Sequence
    (:then_0
      (bind _asbp_enemy (Utilities|Casting|CastToBP_Enemy OtherActor))
      (Game|Damage|ApplyDamage _asbp_enemy 25.0 (Game|GetPlayerController 0) 0 "/Script/Engine.DamageType"))
    (:then_1
      (bind _asbp_copter (Utilities|Casting|CastToBP_Copter OtherActor))
      (Game|Damage|ApplyDamage _asbp_copter 25.0 (Game|GetPlayerController 0) 0))))

(event EventBeginPlay
  (Actor|SetLifeSpan 2.0))

(fn ConstructionScript)