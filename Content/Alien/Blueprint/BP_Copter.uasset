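; BP_Copter is an alien copter enemy that detects BP_Zhopich through PawnSensing and fires at it.
; Each sighting sets OnSee, snaps the copter to face the target and schedules a Shot after a Speed-based Delay.
; Shot spawns BP_DIldoEnemy at the Shoot component's transform.
; Seeing any other pawn clears OnSee and calls StartPatrolling, though the delayed shot still runs.
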(event OnSeePawn(PawnSensing)
  (params (Pawn :type Pawn%20Object%20Reference))
  (Utilities|FlowControl|Sequence
    (:then_0
      (bind _asbp_zhopich (Utilities|Casting|CastToBP_Zhopich Pawn)
        (:then
          (Variables|Default|Seton%20see true)
          (Transformation|SetActorRotation (Math|Rotator|FindLookatRotation (Transformation|GetActorLocation) (Transformation|GetWorldLocation (Variables|/Script/Engine.Actor|GetRootComponent _asbp_zhopich))) true))
        (:CastFailed
          (Variables|Default|Seton%20see false))))
    (:then_1
      (Utilities|FlowControl|Delay (Variables|Default|GetSpeed) :!label _label)
      (CallFunction|Shot))
    (:then_2
      (if (Variables|Default|Geton%20see)
        (goto _label)
        (else
          (CallFunction|StartPatrolling))))))

(event Custom|Shot
  ;[1 1 1] Shot
  (Game|SpawnActorfromClass "/Game/Alien/Blueprint/Bullet/BP_DIldoEnemy.BP_DIldoEnemy_C" (Transformation|GetWorldTransform (Variables|Default|GetShoot)) "AlwaysSpawn" "MultiplyWithRoot" 0 0))

(event EventBeginPlay
  (|CallParentFunction) ; Этот узел отключен и не будет вызываться.\nПеретащите контакты, чтобы построить функционал.
)

(event Collision|EventActorBeginOverlap
  (params (OtherActor :type Actor%20Object%20Reference)))

(event EventTick
  (params (DeltaSeconds :type Float%20%28single-precision%29))
  (|CallParentFunction DeltaSeconds) ; Этот узел отключен и не будет вызываться.\nПеретащите контакты, чтобы построить функционал.
)

(fn ConstructionScript
  (|CallParentFunction))