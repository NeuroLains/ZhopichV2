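; BP_RatKing is a boss that summons enemies near the player and can be killed through damage.
; When PawnSensing sees a BP_Character, a Delay throttles spawning of an Enemy at a fixed offset from that character's location.
; AnyDamage lowers clamped health initialized from MaxHealth on BeginPlay.
; A delayed Tick polls health and, at zero, flags death and destroys the actor.
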(event OnSeePawn(PawnSensing)
  (params (Pawn :type Pawn%20Object%20Reference))
  ;[1 1 1] See
  (bind _asbp_character (Utilities|Casting|CastToBP_Character Pawn))
  (Utilities|FlowControl|Delay 8.0)
  (Game|SpawnActorfromClass (Variables|Default|GetEnemy) (Math|Transform|MakeTransform (Math|Vector|MakeVector (+ (.x (Transformation|GetActorLocation _asbp_character)) 1.5e+02) (+ (.y (Transformation|GetActorLocation _asbp_character)) 1.5e+02) (+ (.z (Transformation|GetActorLocation _asbp_character)) 1.5e+02)) (Transformation|GetActorRotation _asbp_character) "1.000000,1.000000,1.000000") "Undefined" "MultiplyWithRoot" 0 1.2e+03 0.0 4e+02 3.0 0))

(event Custom|DeathC
  ;[1 1 1] Death
  (Variables|Default|SetDeath true)
  (Actor|DestroyActor))

(event Custom|InitHealt
  ;[1 1 1] Health
  (Variables|Default|SetHealth (Variables|Default|GetMaxHealth)))

(event EventBeginPlay
  (CallFunction|InitHealt))

(event Game|Damage|EventAnyDamage
  (params (Damage :type Float%20%28single-precision%29) (DamageType :type Damage%20Type%20Object%20Reference) (InstigatedBy :type Controller%20Object%20Reference) (DamageCauser :type Actor%20Object%20Reference))
  ;[1 1 1] Damage
  (if (not (Variables|Default|GetDeath))
    (Variables|Default|SetHealth (Math|Float|Clamp(Float) (- (Variables|Default|GetHealth) Damage) 0.0 (Variables|Default|GetMaxHealth)))))

(event EventTick
  (params (DeltaSeconds :type Float%20%28single-precision%29))
  ;[1 1 1] Tick
  (Utilities|FlowControl|Delay 0.2)
  (if (<= (Variables|Default|GetHealth) 0.0)
    (CallFunction|DeathC)))

(fn ConstructionScript)