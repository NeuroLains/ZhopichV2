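; BP_Alien is an alien boss that hurts the player on contact and summons enemies.
; Overlapping its Capsule applies heavy damage to BP_Character.
; When PawnSensing sees BP_Character, a short Delay runs, then an Enemy spawns at a fixed offset from the character's current location, matching its rotation.
; Summons can repeat on later sightings, with no cap on their number.
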(event OnComponentBeginOverlap(Capsule)
  (params (OverlappedComponent :type Primitive%20Component%20Object%20Reference) (OtherActor :type Actor%20Object%20Reference) (OtherComp :type Primitive%20Component%20Object%20Reference) (OtherBodyIndex :type Integer) (bFromSweep :type Boolean) (SweepResult :type Hit%20Result%20Structure%20%28by%20ref%29))
  (bind _asbp_character (Utilities|Casting|CastToBP_Character OtherActor))
  (Game|Damage|ApplyDamage _asbp_character 2e+02 0 0))

(event OnSeePawn(PawnSensing)
  (params (Pawn :type Pawn%20Object%20Reference))
  (bind _asbp_character (Utilities|Casting|CastToBP_Character Pawn))
  (Utilities|FlowControl|Delay 5.0)
  (Game|SpawnActorfromClass (Variables|Default|GetEnemy) (Math|Transform|MakeTransform (Math|Vector|MakeVector (+ (.x (Transformation|GetActorLocation _asbp_character)) 1.5e+02) (+ (.y (Transformation|GetActorLocation _asbp_character)) 1.5e+02) (+ (.z (Transformation|GetActorLocation _asbp_character)) 1.5e+02)) (Transformation|GetActorRotation _asbp_character) "1.000000,1.000000,1.000000") "Undefined" "MultiplyWithRoot" 0 1.2e+03 0.0 4e+02 3.0 0))

(event EventBeginPlay)

(event Collision|EventActorBeginOverlap
  (params (OtherActor :type Actor%20Object%20Reference)))

(event EventTick
  (params (DeltaSeconds :type Float%20%28single-precision%29)))

(fn ConstructionScript)