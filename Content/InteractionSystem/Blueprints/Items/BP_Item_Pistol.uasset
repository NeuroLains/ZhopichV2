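; BP_Item_Pistol is a pistol item in the interaction system that fires a bullet when used.
; UseItem spawns a BP_Bullet at the FireLoc component's world transform, always spawning regardless of collision.
; Item query functions report no fracturing and the first item-type enum entry, while GetMesh returns no value.
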(event EventBeginPlay
  (|CallParentFunction) ; This node is disabled and will not be called.\nDrag off pins to build functionality.
)

(event Collision|EventActorBeginOverlap
  (params (OtherActor :type Actor%20Object%20Reference)))

(event EventTick
  (params (DeltaSeconds :type Float%20%28single-precision%29)))

(event EventUseItem
  ;[0.3926 0.4024 1] Spawn Bullet
  (Game|SpawnActorfromClass "/Game/InteractionSystem/Blueprints/Projectile/BP_Bullet.BP_Bullet_C" (Transformation|GetWorldTransform (Variables|Default|GetFireLoc)) "AlwaysSpawn" "OverrideRootScale" 0 0))

(fn ConstructionScript
  (|CallParentFunction))

(fn GetFractureBool
  (return false))

(fn GetItemType
  (return "NewEnumerator0"))

(fn GetMesh
  (return 0))